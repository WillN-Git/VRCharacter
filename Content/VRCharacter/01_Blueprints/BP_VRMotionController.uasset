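; VR motion controller actor for one hand, with an animated hand mesh, mirrored for the left.
; Each tick derives the grip state from attached actor, grip input and nearby objects, passes it to the hand AnimBP, then calls SetFingerTriggers.
; Per-finger trigger overlaps fill overlap and blocked maps; only the overlap entries clear on exit.
; Overlapping physics-simulating meshes flags them grabbable with a haptic pulse, and hits rumble by impact strength.
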(event OnComponentBeginOverlap(GrabSphereTrigger)
  (params (OverlappedComponent :type Primitive%20Component%20Object%20Reference) (OtherActor :type Actor%20Object%20Reference) (OtherComp :type Primitive%20Component%20Object%20Reference) (OtherBodyIndex :type Integer) (bFromSweep :type Boolean) (SweepResult :type Hit%20Result%20Structure%20%28by%20ref%29))
  ;[0 0 0] Rumble controller when overlapping valid static mesh
  (bind _asstatic_mesh_component (Utilities|Casting|CastToStaticMeshComponent OtherComp))
  (if (Physics|IsSimulatingPhysics _asstatic_mesh_component "None")
    (CallFunction|RumbleController 0.3)
    (Variables|Default|SetbObjectCanBeGrabbed true)))

(event OnComponentEndOverlap(GrabSphereTrigger)
  (params (OverlappedComponent :type Primitive%20Component%20Object%20Reference) (OtherActor :type Actor%20Object%20Reference) (OtherComp :type Primitive%20Component%20Object%20Reference) (OtherBodyIndex :type Integer))
  ;[0 0 0] Rumble controller when overlapping valid static mesh
  (Variables|Default|SetbObjectCanBeGrabbed false))

(event OnComponentEndOverlap(MiddleTrigger3)
  (params (OverlappedComponent :type Primitive%20Component%20Object%20Reference) (OtherActor :type Actor%20Object%20Reference) (OtherComp :type Primitive%20Component%20Object%20Reference) (OtherBodyIndex :type Integer))
  ;[1 0.8238 0.3517] Comment
  (Utilities|Map|Add (Variables|Default|GetFingerTriggersOverlap) "Middle_3" false))

(event OnComponentBeginOverlap(PinkyTrigger3)
  (params (OverlappedComponent :type Primitive%20Component%20Object%20Reference) (OtherActor :type Actor%20Object%20Reference) (OtherComp :type Primitive%20Component%20Object%20Reference) (OtherBodyIndex :type Integer) (bFromSweep :type Boolean) (SweepResult :type Hit%20Result%20Structure%20%28by%20ref%29))
  ;[1 0.8238 0.3517] Comment
  (Utilities|Map|Add (Variables|Default|GetFingerTriggersOverlap) "Pinky_3" true)
  (Utilities|Map|Add (Variables|Default|GetFingerTriggersBlocked) "Pinky_3" true))

(event OnComponentEndOverlap(PinkyTrigger3)
  (params (OverlappedComponent :type Primitive%20Component%20Object%20Reference) (OtherActor :type Actor%20Object%20Reference) (OtherComp :type Primitive%20Component%20Object%20Reference) (OtherBodyIndex :type Integer))
  ;[1 0.8238 0.3517] Comment
  (Utilities|Map|Add (Variables|Default|GetFingerTriggersOverlap) "Pinky_3" false))

(event OnComponentBeginOverlap(ThumbTrigger2)
  (params (OverlappedComponent :type Primitive%20Component%20Object%20Reference) (OtherActor :type Actor%20Object%20Reference) (OtherComp :type Primitive%20Component%20Object%20Reference) (OtherBodyIndex :type Integer) (bFromSweep :type Boolean) (SweepResult :type Hit%20Result%20Structure%20%28by%20ref%29))
  ;[1 0.8238 0.3517] Comment
  (Utilities|Map|Add (Variables|Default|GetFingerTriggersOverlap) "Thumb_2" true)
  (Utilities|Map|Add (Variables|Default|GetFingerTriggersBlocked) "Thumb_2" true))

(event OnComponentEndOverlap(ThumbTrigger2)
  (params (OverlappedComponent :type Primitive%20Component%20Object%20Reference) (OtherActor :type Actor%20Object%20Reference) (OtherComp :type Primitive%20Component%20Object%20Reference) (OtherBodyIndex :type Integer))
  ;[1 0.8238 0.3517] Comment
  (Utilities|Map|Add (Variables|Default|GetFingerTriggersOverlap) "Thumb_2" false))

(event OnComponentBeginOverlap(IndexTrigger2)
  (params (OverlappedComponent :type Primitive%20Component%20Object%20Reference) (OtherActor :type Actor%20Object%20Reference) (OtherComp :type Primitive%20Component%20Object%20Reference) (OtherBodyIndex :type Integer) (bFromSweep :type Boolean) (SweepResult :type Hit%20Result%20Structure%20%28by%20ref%29))
  ;[1 0.8238 0.3517] Comment
  (Utilities|Map|Add (Variables|Default|GetFingerTriggersOverlap) "Index_2" true)
  (Utilities|Map|Add (Variables|Default|GetFingerTriggersBlocked) "Index_2" true))

(event OnComponentEndOverlap(IndexTrigger2)
  (params (OverlappedComponent :type Primitive%20Component%20Object%20Reference) (OtherActor :type Actor%20Object%20Reference) (OtherComp :type Primitive%20Component%20Object%20Reference) (OtherBodyIndex :type Integer))
  ;[1 0.8238 0.3517] Comment
  (Utilities|Map|Add (Variables|Default|GetFingerTriggersOverlap) "Index_2" false))

(event OnComponentBeginOverlap(MiddleTrigger2)
  (params (OverlappedComponent :type Primitive%20Component%20Object%20Reference) (OtherActor :type Actor%20Object%20Reference) (OtherComp :type Primitive%20Component%20Object%20Reference) (OtherBodyIndex :type Integer) (bFromSweep :type Boolean) (SweepResult :type Hit%20Result%20Structure%20%28by%20ref%29))
  ;[1 0.8238 0.3517] Comment
  (Utilities|Map|Add (Variables|Default|GetFingerTriggersOverlap) "Middle_2" true)
  (Utilities|Map|Add (Variables|Default|GetFingerTriggersBlocked) "Middle_2" true))

(event OnComponentEndOverlap(MiddleTrigger2)
  (params (OverlappedComponent :type Primitive%20Component%20Object%20Reference) (OtherActor :type Actor%20Object%20Reference) (OtherComp :type Primitive%20Component%20Object%20Reference) (OtherBodyIndex :type Integer))
  ;[1 0.8238 0.3517] Comment
  (Utilities|Map|Add (Variables|Default|GetFingerTriggersOverlap) "Middle_2" false))

(event OnComponentBeginOverlap(RingTrigger2)
  (params (OverlappedComponent :type Primitive%20Component%20Object%20Reference) (OtherActor :type Actor%20Object%20Reference) (OtherComp :type Primitive%20Component%20Object%20Reference) (OtherBodyIndex :type Integer) (bFromSweep :type Boolean) (SweepResult :type Hit%20Result%20Structure%20%28by%20ref%29))
  ;[1 0.8238 0.3517] Comment
  (Utilities|Map|Add (Variables|Default|GetFingerTriggersOverlap) "Ring_2" true)
  (Utilities|Map|Add (Variables|Default|GetFingerTriggersBlocked) "Ring_2" true))

(event OnComponentBeginOverlap(ThumbTrigger3)
  (params (OverlappedComponent :type Primitive%20Component%20Object%20Reference) (OtherActor :type Actor%20Object%20Reference) (OtherComp :type Primitive%20Component%20Object%20Reference) (OtherBodyIndex :type Integer) (bFromSweep :type Boolean) (SweepResult :type Hit%20Result%20Structure%20%28by%20ref%29))
  ;[1 0.8238 0.3517] Comment
  (Utilities|Map|Add (Variables|Default|GetFingerTriggersOverlap) "Thumb_3" true)
  (Utilities|Map|Add (Variables|Default|GetFingerTriggersBlocked) "Thumb_3" true))

(event OnComponentEndOverlap(RingTrigger2)
  (params (OverlappedComponent :type Primitive%20Component%20Object%20Reference) (OtherActor :type Actor%20Object%20Reference) (OtherComp :type Primitive%20Component%20Object%20Reference) (OtherBodyIndex :type Integer))
  ;[1 0.8238 0.3517] Comment
  (Utilities|Map|Add (Variables|Default|GetFingerTriggersOverlap) "Ring_2" false))

(event OnComponentBeginOverlap(PinkyTrigger2)
  (params (OverlappedComponent :type Primitive%20Component%20Object%20Reference) (OtherActor :type Actor%20Object%20Reference) (OtherComp :type Primitive%20Component%20Object%20Reference) (OtherBodyIndex :type Integer) (bFromSweep :type Boolean) (SweepResult :type Hit%20Result%20Structure%20%28by%20ref%29))
  ;[1 0.8238 0.3517] Comment
  (Utilities|Map|Add (Variables|Default|GetFingerTriggersOverlap) "Pinky_2" true)
  (Utilities|Map|Add (Variables|Default|GetFingerTriggersBlocked) "Pinky_2" true))

(event OnComponentEndOverlap(PinkyTrigger2)
  (params (OverlappedComponent :type Primitive%20Component%20Object%20Reference) (OtherActor :type Actor%20Object%20Reference) (OtherComp :type Primitive%20Component%20Object%20Reference) (OtherBodyIndex :type Integer))
  ;[1 0.8238 0.3517] Comment
  (Utilities|Map|Add (Variables|Default|GetFingerTriggersOverlap) "Pinky_2" false))

(event OnComponentEndOverlap(ThumbTrigger3)
  (params (OverlappedComponent :type Primitive%20Component%20Object%20Reference) (OtherActor :type Actor%20Object%20Reference) (OtherComp :type Primitive%20Component%20Object%20Reference) (OtherBodyIndex :type Integer))
  ;[1 0.8238 0.3517] Comment
  (Utilities|Map|Add (Variables|Default|GetFingerTriggersOverlap) "Thumb_3" false))

(event OnComponentBeginOverlap(IndexTrigger3)
  (params (OverlappedComponent :type Primitive%20Component%20Object%20Reference) (OtherActor :type Actor%20Object%20Reference) (OtherComp :type Primitive%20Component%20Object%20Reference) (OtherBodyIndex :type Integer) (bFromSweep :type Boolean) (SweepResult :type Hit%20Result%20Structure%20%28by%20ref%29))
  ;[1 0.8238 0.3517] Comment
  (Utilities|Map|Add (Variables|Default|GetFingerTriggersOverlap) "Index_3" true)
  (Utilities|Map|Add (Variables|Default|GetFingerTriggersBlocked) "Index_3" true))

(event OnComponentHit(MotionController)
  (params (HitComponent :type Primitive%20Component%20Object%20Reference) (OtherActor :type Actor%20Object%20Reference) (OtherComp :type Primitive%20Component%20Object%20Reference) (NormalImpulse :type Vector :default "0, 0, 0") (Hit :type Hit%20Result%20Structure%20%28by%20ref%29))
  ;[0 0 0] Rumble controller when hit another component
  (CallFunction|RumbleController (Math|Float|MapRangeClamped (Math|Vector|VectorLength NormalImpulse) 0.0 1e+04 0.0 0.8)))

(event OnComponentEndOverlap(IndexTrigger3)
  (params (OverlappedComponent :type Primitive%20Component%20Object%20Reference) (OtherActor :type Actor%20Object%20Reference) (OtherComp :type Primitive%20Component%20Object%20Reference) (OtherBodyIndex :type Integer))
  ;[1 0.8238 0.3517] Comment
  (Utilities|Map|Add (Variables|Default|GetFingerTriggersOverlap) "Index_3" false))

(event OnComponentBeginOverlap(RingTrigger3)
  (params (OverlappedComponent :type Primitive%20Component%20Object%20Reference) (OtherActor :type Actor%20Object%20Reference) (OtherComp :type Primitive%20Component%20Object%20Reference) (OtherBodyIndex :type Integer) (bFromSweep :type Boolean) (SweepResult :type Hit%20Result%20Structure%20%28by%20ref%29))
  ;[1 0.8238 0.3517] Comment
  (Utilities|Map|Add (Variables|Default|GetFingerTriggersOverlap) "Ring_3" true)
  (Utilities|Map|Add (Variables|Default|GetFingerTriggersBlocked) "Ring_3" true))

(event OnComponentEndOverlap(RingTrigger3)
  (params (OverlappedComponent :type Primitive%20Component%20Object%20Reference) (OtherActor :type Actor%20Object%20Reference) (OtherComp :type Primitive%20Component%20Object%20Reference) (OtherBodyIndex :type Integer))
  ;[1 0.8238 0.3517] Comment
  (Utilities|Map|Add (Variables|Default|GetFingerTriggersOverlap) "Ring_3" false))

(event OnComponentBeginOverlap(MiddleTrigger3)
  (params (OverlappedComponent :type Primitive%20Component%20Object%20Reference) (OtherActor :type Actor%20Object%20Reference) (OtherComp :type Primitive%20Component%20Object%20Reference) (OtherBodyIndex :type Integer) (bFromSweep :type Boolean) (SweepResult :type Hit%20Result%20Structure%20%28by%20ref%29))
  ;[1 0.8238 0.3517] Comment
  (Utilities|Map|Add (Variables|Default|GetFingerTriggersOverlap) "Middle_3" true)
  (Utilities|Map|Add (Variables|Default|GetFingerTriggersBlocked) "Middle_3" true))

(event Custom|RumbleController
  (params (Intensity :type Float%20%28double-precision%29))
  ;[1 1 1] Rumble Control Event
  (Class|PlayerController|PlayHapticEffect (Game|GetPlayerController 0) "/Game/VRCharacter/10_Settings/Miscellaneous/MotionControllerHaptics.MotionControllerHaptics" (Variables|Default|GetHand) Intensity false))

(event Custom|Update%20Hand%20Animation
  ;[1 1 1] Update Hand Animation
  (Utilities|FlowControl|Sequence
    (:then_0
      ;;[0.4549 0.4549 0.4549] Update Grip State
      (if (or (!= (Variables|Default|GetAttachedActor) 0) (Variables|Default|GetbWantToGrip))
        (Variables|Default|SetGripState "Grab")
        (else
          (bind _returnvalue (Class|VRMotionController|ObjectSelection)) ; Returns the nearest mesh that's overlapping the hand
          (if (!= _returnvalue 0)
            (Variables|Default|SetGripState "CanGrab")
            (elif (Variables|Default|GetbWantToGrip)
              (Variables|Default|SetGripState "Grab")
              (else
                (Variables|Default|SetGripState "Open")))))))
    (:then_1
      ;;[0.4549 0.4549 0.4549] Update Hand Animation state
      (bind _asabp_qk_custom_hand (Utilities|Casting|CastToABP_QK_CustomHand (Components|SkeletalMesh|GetAnimInstance (Variables|Default|GetHandSkeletalMesh))))
      (Variables|/Game/VRCharacter/05_Animations/ABP_QK_CustomHand.ABP_QK_CustomHand_C|SetGripState _asabp_qk_custom_hand (Variables|Default|GetGripState)))))

(event EventBeginPlay
  ;[0 0 0] Create the left hand
  (switch Utilities|FlowControl|Switch|SwitchonEControllerHand (Variables|Default|GetHand)
    (:Left
      (Transformation|SetWorldScale3D (Variables|Default|GetHandSkeletalMesh) "1.000000,1.000000,-1.000000"))))

(event EventTick
  (params (DeltaSeconds :type Float%20%28single-precision%29))
  ;[0 0 0] Main Loop (Tick)
  (Utilities|FlowControl|Sequence
    (:then_0
      (CallFunction|UpdateHandAnimation))
    (:then_1
      (Class|VRMotionController|SetFingerTriggers))))

(fn ConstructionScript
  ;[0 0 0] Update motion source
  (Variables|/Script/HeadMountedDisplay.MotionControllerComponent|SetMotionSource (Variables|Default|GetMotionController) (Utilities|Name|EnumtoName (Variables|Default|GetHand))))

(fn PlaceBoneTriggers)